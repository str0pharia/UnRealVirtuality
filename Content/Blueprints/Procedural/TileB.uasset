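; TileB is a procedural track tile that places an obstacle and chains to the next tile as the AirBalloon travels.
; Construction caches the world transforms of three spawn points, and BeginPlay passes a random one as the relative transform of a child actor obstacle.
; GetAttachTransform exposes the AttachPoint's world transform.
; When AirBalloon overlaps the End component, the game mode adds a tile and this one destroys itself after a short delay.
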(event OnComponentBeginOverlap(End)
  (params (OverlappedComponent :type Primitive%20Component%20Object%20Reference) (OtherActor :type Actor%20Object%20Reference) (OtherComp :type Primitive%20Component%20Object%20Reference) (OtherBodyIndex :type Integer) (bFromSweep :type Boolean) (SweepResult :type Hit%20Result%20Structure%20%28by%20ref%29))
  (Utilities|Casting|CastToAirBalloon OtherActor)
  (bind _asun_real_virtuality_game_mode_bp (Utilities|Casting|CastToUnRealVirtualityGameMode_BP (Game|GetGameMode)))
  (Default|AddTile _asun_real_virtuality_game_mode_bp)
  (Utilities|FlowControl|Delay 0.2)
  (Actor|DestroyActor))

(event EventBeginPlay
  (CallFunction|SpawnObstacle))

(event Collision|EventActorBeginOverlap
  (params (OtherActor :type Actor%20Object%20Reference)))

(event EventTick
  (params (DeltaSeconds :type Float%20%28single-precision%29)))

(fn ConstructionScript
  (bind _spawnpoints (CallFunction|GetSpawnPoints))
  (Variables|Default|SetSpawnPoints _spawnpoints))

(fn GetAttachTransform
  (return (Transformation|GetWorldTransform (Variables|Default|GetAttachPoint))))

(fn GetSpawnPoints
  (return (Utilities|Array|MakeArray (Transformation|GetWorldTransform (Variables|Default|GetSpawnPointA)) (Transformation|GetWorldTransform (Variables|Default|GetSpawnPointB)) (Transformation|GetWorldTransform (Variables|Default|GetSpawnPointC)))))

(fn SpawnObstacle
  (bind _spawnpoints (Variables|Default|GetSpawnPoints))
  (AddComponent|AddChildActorComponent false (Utilities|Array|Get(acopy) _spawnpoints (Math|Random|RandomIntegerinRange 0 (Utilities|Array|LastIndex _spawnpoints)))))