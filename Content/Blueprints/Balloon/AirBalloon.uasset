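; Physics-driven hot air balloon actor with a pull handle that a hand-tagged component grabs by overlap to throttle lift.
; Once a character reference is set, Tick applies constant up and forward forces plus wind to the balloon.
; While the handle is held, Throttle adds upward force proportional to its distance from the physics constraint and prints that distance.
; A Strafe function for sideways force exists but is disconnected.
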(event OnComponentBeginOverlap(Handle)
  (params (OverlappedComponent :type Primitive%20Component%20Object%20Reference) (OtherActor :type Actor%20Object%20Reference) (OtherComp :type Primitive%20Component%20Object%20Reference) (OtherBodyIndex :type Integer) (bFromSweep :type Boolean) (SweepResult :type Hit%20Result%20Structure%20%28by%20ref%29))
  (if (Components|ComponentHasTag OtherComp "hand")
    (Variables|Default|SetPullHandle true)))

(event OnComponentEndOverlap(Handle)
  (params (OverlappedComponent :type Primitive%20Component%20Object%20Reference) (OtherActor :type Actor%20Object%20Reference) (OtherComp :type Primitive%20Component%20Object%20Reference) (OtherBodyIndex :type Integer))
  (if (Components|ComponentHasTag OtherComp "hand")
    (Variables|Default|SetPullHandle false)))

(event EventBeginPlay)

(event Collision|EventActorBeginOverlap
  (params (OtherActor :type Actor%20Object%20Reference)))

(event EventTick
  (params (DeltaSeconds :type Float%20%28single-precision%29))
  (if (Utilities|IsValid (Variables|Default|GetCharacter))
    (CallFunction|Movement)
    (if (Variables|Default|GetPullHandle)
      (CallFunction|Throttle))))

(fn ConstructionScript
  (Variables|Default|SetTankSlotRight (Variables|Default|GetTankSlotRight))
  (Variables|Default|SetTankSlotLeft (Variables|Default|GetTankSlotLeft)))

(fn GetBasket
  (return (Variables|Default|GetBasket)))

(fn Throttle
  (bind _handle (Variables|Default|GetHandle))
  (bind _physicsconstraint1 (Variables|Default|GetPhysicsConstraint1))
  (bind _returnvalue (Transformation|GetWorldLocation _handle))
  (bind _returnvalue_2 (Transformation|GetWorldLocation _physicsconstraint1))
  (bind _returnvalue_3 (- _returnvalue_2 _returnvalue))
  (bind _returnvalue_4 (Math|Vector|VectorLength _returnvalue_3))
  (Development|PrintString (Utilities|String|ToString(Float) _returnvalue_4) true false)
  (Physics|AddForce (Variables|Default|GetBalloon) (* (Math|Vector|Normalize (Transformation|GetActorUpVector self)) (* _returnvalue_4 (Variables|Default|GetForceScalar_Throttle))) "None" false))

(fn Strafe
  (params (DeltaTime :type Float%20%28single-precision%29))
  (bind _returnvalue (Transformation|GetActorRightVector))
  (bind _forcescalar_strafe (Variables|Default|GetForceScalar_Strafe))
  (if (Variables|/Game/EpicTemplates/VRTemplate/Blueprints/MotionControllerPawn.MotionControllerPawn_C|GetStrafeLeft (Variables|Default|GetCharacter))
    (Class|PrimitiveComponent|AddForceatLocation (Variables|Default|GetBalloon) (* (* _returnvalue -1.0) _forcescalar_strafe) (Transformation|GetWorldLocation (Variables|Default|GetMiddle)) "None")
    (else
      (Physics|AddForce (Variables|Default|GetBalloon) (* _returnvalue _forcescalar_strafe) "None" false))))

(fn SetCharacterReference
  (params (Character%20Ref :type Motion%20Controller%20Pawn%20Object%20Reference))
  (Variables|Default|SetCharacter Character%20Ref))

(fn GetOrigin
  (return (Transformation|GetWorldLocation (Variables|Default|GetOrigin))))

(fn Movement
  (bind _balloon (Variables|Default|GetBalloon))
  (Physics|AddForce _balloon (* (Transformation|GetActorUpVector) (Variables|Default|GetForceScalar_Up)) "None" false)
  (Physics|AddForce _balloon (* (Transformation|GetActorForwardVector) (Variables|Default|GetForceScalar_Fwd)) "None" false)
  (Physics|AddForce _balloon (* (Variables|Default|GetWind%20Direction) (* (Variables|Default|GetWind%20Speed%20Scalar) (Variables|Default|GetWind%20Strength%20Scalar))) "None" false))