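; VRPlayer is the VR player Blueprint that rides in the basket of an AirBalloon.
; On BeginPlay it sets floor-level tracking, takes the last AirBalloon found in the level and snaps to its basket's MidFloorSocket, keeping world rotation.
; The construction script enables seated and hands-only flags, and two helpers return HMD device position and head world location.
; The parent BeginPlay is not called.
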(event EventBeginPlay
  (Class|HeadMountedDisplayFunctionLibrary|SetTrackingOrigin "Floor")
  (bind _outactors (Actor|GetAllActorsOfClass "/Game/Blueprints/Balloon/AirBalloon.AirBalloon_C"))
  (for _array_element _outactors
    (bind _output_get (Variables|Default|Setballoon_0 _array_element)))
  (bind _basket_mesh (Default|GetBasket _output_get))
  (Transformation|AttachComponentToComponent self _basket_mesh "MidFloorSocket" "SnapToTarget" "KeepWorld" "KeepWorld" true))

(event Collision|EventActorBeginOverlap
  (params (OtherActor :type Actor%20Object%20Reference)))

(event EventTick
  (params (DeltaSeconds :type Float%20%28single-precision%29))
  (|CallParentFunction DeltaSeconds) ; This node is disabled and will not be called.\nDrag off pins to build functionality.
)

(fn ConstructionScript
  (Variables|Default|Setseated true)
  (Variables|Default|Sethands%20only true))

(fn GetHmdLocation
  (return (.DevicePosition (Class|HeadMountedDisplayFunctionLibrary|GetOrientationandPosition))))

(fn GetHeadLocation
  (return (Transformation|GetWorldLocation (Variables|Default|Getheadscene))))