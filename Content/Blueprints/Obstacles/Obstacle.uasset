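; Obstacle declares a common set of functions for obstacles, with every body empty or returning only a default.
; Queries cover obstacle type, state, score value, wind influence, player detection, actor following and a line-of-sight range for a given direction.
; ObstacleEvent, SwitchState and Update are hooks for behavior, with no logic in this asset.
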(fn IsAffectedbyWind
  (return false))

(fn GetScoreValue
  (return 0.0))

(fn GetObstacleState)

(fn PlayerDetected
  (return false))

(fn IsFollowingActor
  (return false 0))

(fn ObstacleEvent)

(fn SwitchState)

(fn LosRange
  (params (Direction :type Vector))
  (return 0.0))

(fn Update)

(fn GetObstacleType
  (return "NewEnumerator0"))