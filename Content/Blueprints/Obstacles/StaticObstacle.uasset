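; StaticObstacle is an obstacle actor Blueprint with no behavior of its own, as its event graph and construction script are empty.
; Its query functions report it as non-dynamic, unaffected by wind, not dashing, not following an actor and not detecting the player.
; Follow conditions, safe zone and score values all return zero, so it serves as an inert obstacle answering the common obstacle queries.
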(event EventBeginPlay)

(event Collision|EventActorBeginOverlap
  (params (OtherActor :type Actor%20Object%20Reference)))

(event EventTick
  (params (DeltaSeconds :type Float%20%28single-precision%29)))

(fn ConstructionScript)

(fn GetFollowActorConditions
  (return 0.0 0.0))

(fn GetSafeZone
  (return 0.0 "0, 0, 0"))

(fn GetScoreValues
  (return 0.0 0.0 0.0 0.0))

(fn IsAffectedbyWind
  (return false))

(fn IsDashing
  (return false))

(fn IsDynamic
  (return false))

(fn IsFollowingActor
  (return false 0))

(fn PlayerDetected
  (return false))